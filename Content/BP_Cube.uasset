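; BP_Cube is a trigger cube that awards the player a point on overlap.
; When a BP_Player begins overlapping BoxCollision, it increments that player's Score and prints the new value, with no guard against repeat overlaps.
; An uncalled PrintScore function repeats this logic but casts the box's own owner to BP_Player instead of the overlapping actor.
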(event `self.BoxCollision.OnComponentBeginOverlap`
  (params (OverlappedComponent :type "PrimitiveComponent Object Reference") (OtherActor :type "Actor Object Reference") (OtherComp :type "PrimitiveComponent Object Reference") (OtherBodyIndex :type Integer) (bFromSweep :type Boolean) (SweepResult :type "HitResult Structure (by ref)"))
  (bind _asbp_player (cast `/Game/BP_Player` OtherActor))
  (bind _output_get (set `/Game/BP_Player.Score` (+ (`/Game/BP_Player.Score` _asbp_player) 1) _asbp_player))
  (`KismetSystemLibrary.PrintString` (`KismetStringLibrary.Conv_IntToString` _output_get)))

(fn `PrintScore`
  (bind _asbp_player (cast `/Game/BP_Player` (`ActorComponent.GetOwner` (`self.BoxCollision`))))
  (bind _output_get (set `/Game/BP_Player.Score` (+ (`/Game/BP_Player.Score` _asbp_player) 1) _asbp_player))
  (`KismetSystemLibrary.PrintString` (`KismetStringLibrary.Conv_IntToString` _output_get)))

(fn `UserConstructionScript`)